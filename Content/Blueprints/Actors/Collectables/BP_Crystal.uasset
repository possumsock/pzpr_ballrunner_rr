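; BP_Crystal is a collectable crystal that flies into the player and disappears when touched.
; An overlap passing the IsPlayer check caches the crystal's location and plays a timeline.
; Each update lerps the crystal from that start toward the player pawn's current location, homing on a moving player, while a second track shrinks it to zero.
; The actor destroys itself when the timeline finishes, with no score or inventory logic.
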(event Collision|EventActorBeginOverlap
  (params (OtherActor :type Actor%20Object%20Reference))
  (if (.IsPlayer (Utilities|IsPlayer false OtherActor))
    (bind _output_get (CallFunction|GetPlayerPsition))
    (bind (_direction _position _scale) (Timeline|Timeline_0 Play)
      (:Update
        (CallFunction|TeleportingtoPlayer _output_get _position (Game|Player|GetPlayerPawn 0))
        (CallFunction|ActorScale _scale))
      (:Finished
        (Actor|DestroyActor)))))

(fn ConstructionScript)

(fn TeleportingtoPlayer
  (params (A :type Vector) (Alpha :type Float%20%28single-precision%29) (self2 :type Actor%20Object%20Reference))
  (Transformation|SetActorLocation (Math|Vector|Lerp(Vector) A (Transformation|GetActorLocation self2) Alpha) false false))

(fn GetPlayerPsition
  (bind _output_get (Variables|Default|SetLerpStartLocation (Transformation|GetActorLocation)))
  (return _output_get))

(fn ActorScale
  (params (Alpha :type Float%20%28single-precision%29))
  (Transformation|SetActorScale3D (Math|Vector|Lerp(Vector) "1.000000,1.000000,1.000000" "0, 0, 0" Alpha)))